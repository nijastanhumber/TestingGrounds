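; AI controller for guard NPCs that runs the GuardBehaviour tree on the PatrolData blackboard at BeginPlay.
; AI Perception updates store sensed actors without the "Enemy" tag in the blackboard's enemy key and clear it when sensing is lost.
; Each tick, it sets the controlled TP_Character's Aiming and Shooting flags according to whether the controller has a valid focus actor.
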(event OnTargetPerceptionUpdated(AIPerception)
  (params (Actor :type Actor%20Object%20Reference) (Stimulus :type AI%20Stimulus%20Structure))
  (bind _enemykey (Variables|Default|GetEnemyKey))
  (bind _blackboardref (Variables|Default|GetBlackboardRef))
  (if (not (Actor|ActorHasTag Actor "Enemy"))
    (if (.bSuccessfullySensed (Utilities|Struct|BreakAIStimulus Stimulus))
      (AI|Components|Blackboard|SetValueasObject _blackboardref _enemykey Actor)
      (else
        (AI|Components|Blackboard|ClearValue _blackboardref _enemykey)))))

(event EventBeginPlay
  (bind _blackboardcomponent (Class|AIController|UseBlackboard "/Game/Dynamic/NPC/AI/PatrolData.PatrolData"))
  (AI|RunBehaviorTree "/Game/Dynamic/NPC/AI/GuardBehaviour.GuardBehaviour")
  (Variables|Default|SetBlackboardRef _blackboardcomponent))

(event EventTick
  (params (DeltaSeconds :type Float%20%28single-precision%29))
  (bind _returnvalue (Class|AIController|GetFocusActor))
  (bind _returnvalue_2 (Utilities|IsValid _returnvalue))
  (bind _astp_character (Utilities|Casting|CastToTP_Character (Pawn|GetControlledPawn)))
  (Variables|/Game/Dynamic/NPC/Behaviour/TP_Character.TP_Character_C|SetAiming _astp_character _returnvalue_2)
  (Variables|/Game/Dynamic/NPC/Behaviour/TP_Character.TP_Character_C|SetShooting _astp_character _returnvalue_2))

(fn ConstructionScript)