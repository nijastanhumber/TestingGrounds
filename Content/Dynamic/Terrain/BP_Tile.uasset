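; BP_Tile is an infinite-terrain tile that populates itself on BeginPlay with random props and AI enemies via PlaceActors and PlaceAIPawns.
; The player entering LockingVolume turns the barrier green and passable and reports the tile conquered to the game mode once; leaving turns it red and solid.
; Player overlap with DestroyVolume makes the game mode spawn another tile and destroys this one.
; An arrow component supplies the attach transform.
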(event OnComponentBeginOverlap(LockingVolume)
  (params (OverlappedComponent :type Primitive%20Component%20Object%20Reference) (OtherActor :type Actor%20Object%20Reference) (OtherComp :type Primitive%20Component%20Object%20Reference) (OtherBodyIndex :type Integer) (bFromSweep :type Boolean) (SweepResult :type Hit%20Result%20Structure%20%28by%20ref%29))
  (if (== OtherActor (Game|GetPlayerCharacter 0))
    (Utilities|FlowControl|Sequence
      (:then_0
        (CallFunction|Unlock))
      (:then_1
        (CallFunction|TileConquered)))))

(event OnComponentEndOverlap(LockingVolume)
  (params (OverlappedComponent :type Primitive%20Component%20Object%20Reference) (OtherActor :type Actor%20Object%20Reference) (OtherComp :type Primitive%20Component%20Object%20Reference) (OtherBodyIndex :type Integer))
  (if (== OtherActor (Game|GetPlayerCharacter 0))
    (CallFunction|Lock)))

(event OnComponentBeginOverlap(DestroyVolume)
  (params (OverlappedComponent :type Primitive%20Component%20Object%20Reference) (OtherActor :type Actor%20Object%20Reference) (OtherComp :type Primitive%20Component%20Object%20Reference) (OtherBodyIndex :type Integer) (bFromSweep :type Boolean) (SweepResult :type Hit%20Result%20Structure%20%28by%20ref%29))
  (if (== OtherActor (Game|GetPlayerCharacter 0))
    (bind _asbp_infinite_terrain_game_mode (Utilities|Casting|CastToBP_InfiniteTerrainGameMode (Game|GetGameMode)))
    (Default|SpawnTile _asbp_infinite_terrain_game_mode)
    (Actor|DestroyActor)))

(event EventBeginPlay
  (CallFunction|Unlock)
  (Class|Tile|PlaceActors "/Game/Dynamic/Terrain/Props/BP_Container.BP_Container_C" 1 3 4e+02 1.0 1.0)
  (Class|Tile|PlaceActors "/Game/Dynamic/Terrain/Props/BP_Box.BP_Box_C" 2 4 1e+02 1.0 1.0)
  (Class|Tile|PlaceActors "/Game/Dynamic/Terrain/Props/BP_Canister.BP_Canister_C" 1 7 5e+01 1.0 1.0)
  (Class|Tile|PlaceActors "/Game/Dynamic/Terrain/Props/BP_Rock1.BP_Rock1_C" 1 4 1.5e+02 1.0 5.0)
  (Class|Tile|PlaceActors "/Game/Dynamic/Terrain/Props/BP_Rock2.BP_Rock2_C" 1 4 2.5e+02 1.0 5.0)
  (Class|Tile|PlaceActors "/Game/Dynamic/Terrain/Props/BP_Rock3.BP_Rock3_C" 1 4 2.5e+02 1.0 5.0)
  (Class|Tile|PlaceActors "/Game/Dynamic/Terrain/Props/BP_SandBags.BP_SandBags_C" 1 2 2.5e+02 1.0 1.0)
  (Class|Tile|PlaceAIPawns "/Game/Dynamic/Character/Behaviour/BP_Character.BP_Character_C" (Variables|Default|GetMinEnemies) (Variables|Default|GetMaxEnemies) 1e+02))

(event Collision|EventActorBeginOverlap
  (params (OtherActor :type Actor%20Object%20Reference)))

(event EventTick
  (params (DeltaSeconds :type Float%20%28single-precision%29)))

(fn ConstructionScript)

(fn GetAttachLocation
  (return (Transformation|GetWorldTransform (Variables|Default|GetArrow))))

(fn Lock
  (Collision|SetCollisionEnabled (Variables|Default|GetBlockingWall) "QueryAndPhysics")
  (Rendering|Material|SetMaterial (Variables|Default|GetBlockingWall) 0 "/Game/Dynamic/Terrain/MI_Barrier_Red.MI_Barrier_Red"))

(fn Unlock
  (Collision|SetCollisionEnabled (Variables|Default|GetBlockingWall) "NoCollision")
  (Rendering|Material|SetMaterial (Variables|Default|GetBlockingWall) 0 "/Game/Dynamic/Terrain/MI_Barrier_Green.MI_Barrier_Green"))

(fn TileConquered
  (if (not (Variables|Default|GetIsTileConquered))
    (Default|NewTileConquered (.AsBP%20Infinite%20Terrain%20Game%20Mode (Utilities|Casting|CastToBP_InfiniteTerrainGameMode (Game|GetGameMode))))
    (Variables|Default|SetIsTileConquered true)))